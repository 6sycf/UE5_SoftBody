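; BP_Debug is a debug Blueprint for testing mouse picking of vertices on a soft body mesh.
; BeginPlay shows the mouse cursor and caches the MySoftBodyMeshComponent from a SoftBody actor found in the level.
; Left click deprojects the cursor into a world ray, passes it to SelectVertexByRay with a fixed click tolerance, and prints the result.
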(event EventBeginPlay
  (Variables|Default|SetbShowMouseCursor true)
  (bind _returnvalue (Actor|GetActorOfClass "/Game/蓝图/SoftBody.SoftBody_C"))
  (Variables|Default|SetNewVar (Actor|GetComponentbyClass _returnvalue "/Script/SoftBody.MySoftBodyMeshComponent")))

(event EventTick
  (params (DeltaSeconds :type Float%20%28single-precision%29)))

(event Input|MouseEvents|LeftMouseButton
  (params (Key :type Key%20Structure :default "None"))
  (bind _returnvalue (Game|GetPlayerController 0))
  (bind (_worldlocation _worlddirection _returnvalue_2) (Game|Player|ConvertMouseLocationToWorldSpace _returnvalue))
  (:Pressed
    (if _returnvalue_2
      (bind _returnvalue_3 (Class|MySoftBodyMeshComponent|SelectVertexbyRay (Variables|Default|GetNewVar) _worldlocation _worlddirection 5e+01))
      (Development|PrintString (Utilities|String|ToString(Integer) _returnvalue_3)))))

(fn ConstructionScript)